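; Player character Blueprint that owns the player's HUD, crafting menu and grid-snap toggle.
; BeginPlay adds the player and objective widgets to the viewport, and ShowResourcePopup forwards resource type and amount to the player widget.
; CraftMenu input creates or removes the crafting widget based on IsCrafting, switching cursor and input mode to match.
; ToggleGridSnap flips UseGridSnap; a debug print of hunger, health and stamina is left unconnected.
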(event `self.ReceiveBeginPlay`
  ; BeginPlay
  (bind _returnvalue (`|CreateWidget` "/Game/Widgets/Player_W.Player_W_C"))
  (bind _output_get (set `self.PlayerUI` _returnvalue))
  (`UserWidget.AddToViewport` _output_get 0)
  (bind _returnvalue_2 (`|CreateWidget` "/Game/Widgets/Objective_W.Objective_W_C"))
  (bind _output_get_2 (set `self.objWidget` _returnvalue_2))
  (`UserWidget.AddToViewport` _output_get_2 0))

(event `self.ShowResourcePopup`
  (params (ResourceType :type String) (Amount :type "Float (single-precision)"))
  ; BeginPlay
  (bind _output_get (set `self.As Player W` (stale `self.ReceiveBeginPlay` _returnvalue)))
  (`/Game/Widgets/Player_W.ResourcePop` _output_get ResourceType Amount))

(event `InputAction|ToggleGridSnap`
  (params (Key :type "Key Structure"))
  ; ToggleSnap
  (:`Pressed`
    (`/Engine/EditorBlueprintResources/StandardMacros.FlipFlop`
      (:`A`
        (set `self.bUseGridSnap` false))
      (:`B`
        (set `self.bUseGridSnap` true)))))

(event `self.ReceiveTick`
  (params (DeltaSeconds :type "Float (single-precision)"))
  ; Debug
)

(event `InputAction|CraftMenu`
  (params (Key :type "Key Structure"))
  (bind _returnvalue (`GameplayStatics.GetPlayerController` 0))
  (bind _iscrafting (`self.isCrafting`))
  ; CraftingMenu
  (:`Pressed`
    (`/Engine/EditorBlueprintResources/StandardMacros.FlipFlop`
      (:`A`
        (if _iscrafting
          (`Widget.RemoveFromParent` (stale _returnvalue_2) :!label _label)
          (set `PlayerController.bShowMouseCursor` false _returnvalue)
          (`WidgetBlueprintLibrary.SetInputMode_GameOnly` _returnvalue)
          (`WidgetBlueprintLibrary.SetFocusToGameViewport`)
          (set `self.isCrafting` false)
          (else
            (bind _returnvalue_2 (`|CreateWidget` "/Game/Widgets/Crafting_W.Crafting_W_C" :!label _label_2))
            (`UserWidget.AddToViewport` _returnvalue_2 0)
            (set `PlayerController.bShowMouseCursor` true _returnvalue)
            (`WidgetBlueprintLibrary.SetInputMode_GameAndUIEx` _returnvalue _returnvalue_2)
            (set `self.isCrafting` true))))
      (:`B`
        (if _iscrafting
          (goto _label)
          (else
            (goto _label_2)))))))

(fn `UserConstructionScript`)